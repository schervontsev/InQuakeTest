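; PlayerState_DM is a player state, apparently for a deathmatch mode, that tracks a player's frag count.
; AddFrag runs only with authority, incrementing Frags and comparing it to the FragLimit held by GameState_DM.
; When the limit is reached, it calls EndGame on GameMode_DM to finish the match.
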(event `self.ReceiveTick`
  (params (DeltaSeconds :type "Float (single-precision)")))

(fn `AddFrag`
  (`/Engine/EditorBlueprintResources/ActorMacros.Switch Has Authority`
    (:`Authority`
      (bind _result (`/Engine/EditorBlueprintResources/StandardMacros.IncrementInt` (`self.Frags`))
        (:`  `
          (bind _asgame_state_dm (cast `/Game/Blueprints/GameState_DM` (`GameplayStatics.GetGameState`)))
          (if (>= _result (`/Game/Blueprints/GameState_DM.FragLimit` _asgame_state_dm))
            (bind _asgame_mode_dm (cast `/Game/Blueprints/GameMode_DM` (`GameplayStatics.GetGameMode`)))
            (`/Game/Blueprints/GameMode_DM.EndGame` _asgame_mode_dm)))))))

(fn `UserConstructionScript`)