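; Deathmatch game mode that respawns players when they die and ends the match, acting only on the server.
; OnDie destroys the controlled pawn, waits for GameState_DM's RespawnDelay, then spawns a ThirdPersonCharacter at a random PlayerStart and possesses it.
; EndGame sets the GameEnded flag, which blocks further respawns including those waiting on the delay, and forwards the call to GameState_DM.
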(event `self.ReceiveBeginPlay`)

(event `self.ReceiveTick`
  (params (DeltaSeconds :type "Float (single-precision)")))

(event `OnDie`
  (params (PlayerController :type "Controller Object Reference"))
  (`/Engine/EditorBlueprintResources/ActorMacros.Switch Has Authority`
    (:`Authority`
      (bind _outactors (`GameplayStatics.GetAllActorsOfClass` "/Script/Engine.PlayerStart")) ; Get random player start
      (`self.K2_DestroyActor` (`Controller.K2_GetPawn` PlayerController))
      (bind _asgame_state_dm (cast `/Game/Blueprints/GameState_DM` (`GameplayStatics.GetGameState`))
        (:`then`
          (`KismetSystemLibrary.Delay` (`/Game/Blueprints/GameState_DM.RespawnDelay` _asgame_state_dm)) ; pause before respawn
        )
        (:`CastFailed`
          _))
      (if (not (`self.GameEnded`))
        (bind _returnvalue (`|SpawnActorFromClass` "/Game/Blueprints/ThirdPersonCharacter.ThirdPersonCharacter_C" (`self.GetTransform` (`KismetArrayLibrary.Array_Get` _outactors (`KismetMathLibrary.RandomInteger` (`KismetArrayLibrary.Array_Length` _outactors)))) "AdjustIfPossibleButAlwaysSpawn" "OverrideRootScale"))
        (`/Engine/EditorBlueprintResources/StandardMacros.IsValid` _returnvalue
          (:`Is Valid`
            (`Controller.Possess` PlayerController _returnvalue)))))))

(fn `EndGame`
  (`/Engine/EditorBlueprintResources/ActorMacros.Switch Has Authority`
    (:`Authority`
      (set `self.GameEnded` true)
      (bind _asgame_state_dm (cast `/Game/Blueprints/GameState_DM` (`GameplayStatics.GetGameState`)))
      (`/Game/Blueprints/GameState_DM.EndGame` _asgame_state_dm))))

(fn `UserConstructionScript`)