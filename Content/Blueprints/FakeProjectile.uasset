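; Stand-in arrow projectile that flies slowed until the real arrow catches up with it, masking network latency.
; On BeginPlay it sets a timer scaled from the instigator's PlayerState ping, after which RestoreSpeed doubles the ProjectileMovement velocity.
; Overlapping any actor other than the instigator stops its movement immediately.
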(event EventBeginPlay
  (Utilities|Time|SetTimerbyFunctionName 0 "RestoreSpeed" (/ (Math|Conversions|ToFloat(Byte) (Variables|/Script/Engine.PlayerState|GetPing (Variables|/Script/Engine.Pawn|GetPlayerState (Game|GetInstigator)))) 125.0)) ; slow down arrow before real one catches up with it
)

(event EventActorBeginOverlap
  (params (OtherActor :type Actor%20Object%20Reference))
  (if (!= OtherActor (Game|GetInstigator))
    (Components|Movement|StopMovementImmediately (Variables|Default|GetProjectileMovement))))

(fn ConstructionScript
  (|CallParentFunction))

(fn RestoreSpeed
  (bind _projectilemovement (Variables|Default|GetProjectileMovement))
  (Variables|/Script/Engine.MovementComponent|SetVelocity _projectilemovement (* (Variables|/Script/Engine.MovementComponent|GetVelocity _projectilemovement) 2.0)))