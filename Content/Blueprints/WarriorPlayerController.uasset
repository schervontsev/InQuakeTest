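; Player controller for the Warrior player that manages the HUD, the end-of-game screen and quitting.
; On BeginPlay it creates the WarriorHUD widget and keeps a reference to it.
; EndGame removes that HUD, shows EndGameWidget and unpossesses the pawn; Escape quits the game.
; All three paths run only on the Remote branch of an authority check, so they are skipped wherever the controller has authority.
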(event `Key|Escape`
  (params (Key :type "Key Structure" :default "AnyKey"))
  (:`Pressed`
    (`/Engine/EditorBlueprintResources/ActorMacros.Switch Has Authority`
      (:`Remote`
        (`KismetSystemLibrary.QuitGame` null "Quit")))))

(event `self.ReceiveBeginPlay`
  (`/Engine/EditorBlueprintResources/ActorMacros.Switch Has Authority`
    (:`Remote`
      (bind _returnvalue (`|CreateWidget` "/Game/GUI/WarriorHUD.WarriorHUD_C" self))
      (bind _output_get (set `self.HUD` _returnvalue))
      (`UserWidget.AddToViewport` _output_get 0))))

(event `self.ReceiveTick`
  (params (DeltaSeconds :type "Float (single-precision)")))

(fn `EndGame`
  (`/Engine/EditorBlueprintResources/ActorMacros.Switch Has Authority`
    (:`Remote`
      (`Widget.RemoveFromParent` (`self.HUD`))
      (bind _returnvalue (`|CreateWidget` "/Game/GUI/EndGameWidget.EndGameWidget_C" self))
      (`UserWidget.AddToViewport` _returnvalue 0)
      (`self.UnPossess`))))

(fn `UserConstructionScript`)