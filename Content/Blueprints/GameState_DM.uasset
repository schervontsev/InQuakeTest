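; Deathmatch GameState that ends the match and reports the top fragger.
; EndGame loops PlayerArray to each owning WarriorPlayerController, unpossessing it on the authority and calling that controller's EndGame on remotes.
; GetHighestFrags scans the PlayerState_DM entries and returns the highest frag count with that player's name.
; GetWinner is an empty stub.
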(event Custom|EndGame
  (for _array_element (Variables|Default|GetPlayerArray)
    (bind _aswarrior_player_controller (Utilities|Casting|CastToWarriorPlayerController (Components|GetOwner _array_element)))
    (Networking|SwitchHasAuthority
      (:Authority
        (Pawn|UnPossess _aswarrior_player_controller))
      (:Remote
        (Default|EndGame _aswarrior_player_controller)))))

(event EventBeginPlay)

(event EventTick
  (params (DeltaSeconds :type Float%20%28single-precision%29)))

(fn ConstructionScript)

(fn GetHighestFrags
  (for _array_element (Variables|Default|GetPlayerArray)
    (bind _asplayer_state_dm (Utilities|Casting|CastToPlayerState_DM _array_element))
    (if (> (Variables|/Game/Blueprints/PlayerState_DM.PlayerState_DM_C|GetFrags _asplayer_state_dm) (LocalVariables|GetHighestFrags))
      (LocalVariables|SetHighestFrags (Variables|/Game/Blueprints/PlayerState_DM.PlayerState_DM_C|GetFrags _asplayer_state_dm))
      (LocalVariables|SetName (Variables|/Script/Engine.PlayerState|GetPlayerName _asplayer_state_dm))))
  (return (LocalVariables|GetHighestFrags) (LocalVariables|GetName)))

(fn GetWinner)