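; Replicated projectile that damages characters on the server and hides the owning client's lag behind a locally spawned fake projectile.
; On the owner it hides itself, links a free fake from the character, then swaps visibility on a ping-based timer or character overlap.
; Server hits apply the game state's shoot damage and destroy it.
; Otherwise it stops, tears off replication, attaches to any traced pawn and expires on a timer.
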(event `self.ReceiveBeginPlay`
  (bind _returnvalue (`self.GetInstigator`))
  (`/Engine/EditorBlueprintResources/ActorMacros.Switch Has Authority`
    (:`Authority`
      (`KismetSystemLibrary.K2_SetTimer` null "Destroy" (`self.LiveTime`)))
    (:`Remote`
      (if (`Pawn.IsLocallyControlled` _returnvalue)
        (`self.SetActorHiddenInGame` true) ; Use fake projectile on owner, to get instant feedback
        (bind _asthird_person_character (cast `/Game/Blueprints/ThirdPersonCharacter` _returnvalue))
        (bind _freefakeprojectiles (`/Game/Blueprints/ThirdPersonCharacter.FreeFakeProjectiles` _asthird_person_character))
        (bind _item (`KismetArrayLibrary.Array_Get` _freefakeprojectiles))
        (`/Engine/EditorBlueprintResources/StandardMacros.IsValid` _item
          (:`Is Valid`
            (set `self.LinkedFake` _item)
            (`KismetArrayLibrary.Array_Remove` _freefakeprojectiles)
            (`KismetSystemLibrary.K2_SetTimer` null "SyncFake" (/ (`KismetMathLibrary.Conv_ByteToDouble` (`PlayerState.Ping` (`Pawn.PlayerState` (`GameplayStatics.GetPlayerCharacter` 0)))) 125.0)) ; sync projectiles roughly when they went same distance
          ))))))

(event `self.ReceiveActorBeginOverlap`
  (params (OtherActor :type "Actor Object Reference"))
  (bind _returnvalue (`GameplayStatics.GetObjectClass` OtherActor))
  (if (`KismetMathLibrary.ClassIsChildOf` _returnvalue "Projectile_C")
    _
    (elif (`KismetMathLibrary.ClassIsChildOf` _returnvalue "/Game/Blueprints/ThirdPersonCharacter.ThirdPersonCharacter_C")
      (if (!= OtherActor (`self.GetInstigator`))
        (`/Engine/EditorBlueprintResources/ActorMacros.Switch Has Authority`
          (:`Authority`
            ;[1 1 1] Real projectile hit
            (bind _asthird_person_character (cast `/Game/Blueprints/ThirdPersonCharacter` OtherActor))
            (bind _asthird_person_character_2 (cast `/Game/Blueprints/ThirdPersonCharacter` (`self.GetInstigator`)))
            (bind _result (`/Game/Blueprints/ThirdPersonCharacter.GetDMGameState` _asthird_person_character_2))
            (bind _asthird_person_character_3 (cast `/Game/Blueprints/ThirdPersonCharacter` (`self.GetInstigator`)))
            (bind _died (`/Game/Blueprints/ThirdPersonCharacter.TakeDamage` _asthird_person_character (`/Game/Blueprints/GameState_DM.ShootDamage` _result) _asthird_person_character_3))
            (if _died
              (`self.Destroy`)
              (else
                (`self.StopMovement` :!label _label)
                (`self.TearOff`))))
          (:`Remote`
            (if (`Pawn.IsLocallyControlled` (`self.GetInstigator`))
              (`self.SyncFake`)))))
      (else
        (goto _label)))))

(event `StopMovement`
  ;[1 1 1] Stop projectile and try to attach it to hit object
  (`MovementComponent.StopMovementImmediately` (`self.ProjectileMovement`))
  (bind (_outhit _returnvalue) (`KismetSystemLibrary.LineTraceSingleForObjects` (`self.K2_GetActorLocation`) (`SceneComponent.K2_GetComponentLocation` (`self.ArrowEnd`)) (`|MakeArray` "ObjectTypeQuery3" :!type "EObjectTypeQuery Enum")))
  (`self.SetActorEnableCollision` false)
  (if _returnvalue
    (bind (_bblockinghit _binitialoverlap _time _location _impactpoint _normal _impactnormal _physmat _hitactor _hitcomponent _hitbonename) (`GameplayStatics.BreakHitResult` _outhit))
    (`self.K2_AttachRootComponentToActor` _hitactor _hitbonename "KeepWorldPosition" false))
  (`KismetSystemLibrary.K2_SetTimer` null "Destroy" (`self.LiveTimeAfterStop`)))

(event `self.ReceiveTick`
  (params (DeltaSeconds :type "Float (single-precision)")))

(fn `Destroy`
  (`self.SetActorHiddenInGame` true)
  (`self.K2_DestroyActor`))

(fn `SyncFake`
  (bind _linkedfake (`self.LinkedFake`))
  (`/Engine/EditorBlueprintResources/StandardMacros.IsValid` _linkedfake
    (:`Is Valid`
      (`self.SetActorHiddenInGame` _linkedfake true)
      (`self.SetActorEnableCollision` false)
      (`self.SetActorHiddenInGame` false)
      (`self.K2_DestroyActor` _linkedfake))))

(fn `UserConstructionScript`)